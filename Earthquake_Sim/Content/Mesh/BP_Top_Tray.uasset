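; BP_Top_Tray is a tray Blueprint whose Top component slides back and forth between two relative positions, MaxDistA and MaxDistB.
; BeginPlay moves Top to MaxDistA, then starts MoveToB and MoveToA, which call each other in turn after a short pause.
; Each leg uses MoveComponentTo timed by Speed and only runs if Top sits exactly at the opposite endpoint, otherwise the cycle stops.
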(event Custom|MoveToB
  (if (Utilities|Operators|EqualEqual (Variables|/Script/Engine.SceneComponent|GetRelativeLocation (Variables|Default|GetTop)) (Variables|Default|GetMaxDistA) 0.0)
    (Components|MoveComponentTo (Variables|Default|GetTop) (Variables|Default|GetMaxDistB) "0, 0, 0" false false (Variables|Default|GetSpeed) false)
    (Utilities|FlowControl|Delay 0.2)
    (CallFunction|MovetoA)))

(event Custom|MoveToA
  (if (Utilities|Operators|EqualEqual (Variables|/Script/Engine.SceneComponent|GetRelativeLocation (Variables|Default|GetTop)) (Variables|Default|GetMaxDistB) 0.0)
    (Components|MoveComponentTo (Variables|Default|GetTop) (Variables|Default|GetMaxDistA) "0, 0, 0" false false (Variables|Default|GetSpeed) false)
    (Utilities|FlowControl|Delay 0.2)
    (CallFunction|MovetoB)))

(event EventBeginPlay
  (Components|MoveComponentTo (Variables|Default|GetTop) (Variables|Default|GetMaxDistA) "0, 0, 0" false false 0.2 false)
  (Utilities|FlowControl|Delay 0.2)
  (CallFunction|MovetoB))

(fn ConstructionScript)